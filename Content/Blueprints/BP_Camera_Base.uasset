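; Base camera Blueprint with the start of a traveling movement, apparently meant to follow a spline.
; On BeginPlay, if IsActive is set, TravelingMovement plays the Movement timeline, which writes its Alpha track to a variable each update.
; A Lerp over the TravelingRef spline length is left unconnected, so the graph never moves the camera.
; The construction script is empty.
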(event `self.ReceiveBeginPlay`
  ;[0 0 0] CameraMovement
  (if (`self.IsActive?`)
    (`self.TravelingMovement`)))

(event `TravelingMovement`
  (bind (_direction _alpha) (`Timeline|Movement` :`NewTime` 0.0)
    (:`Update`
      (set `self.Alpha` _alpha))))

(fn `UserConstructionScript`)